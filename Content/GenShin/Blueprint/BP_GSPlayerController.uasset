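; Player controller for the GenShin game that manages the score HUD and the end-of-game result screen.
; On BeginPlay it creates the HUD and sets the clear score read from the game mode.
; Score events update the score widget, while game over and game clear share one path that shows a result widget with success or failure.
; Game clear also spawns an actor at the controlled pawn's location.
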(event `self.ReceiveBeginPlay`
  (bind _returnvalue (`|CreateWidget` null))
  (`UserWidget.AddToViewport` _returnvalue 0)
  (set `self.ScoreWidget` (`/Game/GenShin/Blueprint/BP_GSPlayerController.WBP_PlayerScore` _returnvalue))
  (bind _asbp_abgame_mode (cast `` (`GameplayStatics.GetGameMode`)))
  (`self.SetClearScore` (`self.ScoreWidget`) (`/Game/GenShin/Blueprint/BP_GSPlayerController.ClearScore` _asbp_abgame_mode)))

(event `OnNewScore`
  (`self.SetScore` (`self.ScoreWidget`) (stale `self.K2_OnScoreChanged` NewScore) :!label _label))

(event `self.K2_OnScoreChanged`
  (params (NewScore :type Integer))
  (goto _label))

(event `OnGameOver`
  (set `self.Is Success` false :!label _label_2)
  (bind _returnvalue (`|CreateWidget` null (`GameplayStatics.GetPlayerController` 0) :!label _label_3))
  (`UserWidget.AddToViewport` _returnvalue 0)
  (`self.SetResult` _returnvalue (`self.Is Success`)))

(event `self.K2_OnGameOver`
  (goto _label_2))

(event `OnGameClear`
  (set `self.Is Success` true :!label _label_4)
  (`|ExecutionSequence`
    (:`then_0`
      (goto _label_3))
    (:`then_1`
      (`|SpawnActorFromClass` null (`KismetMathLibrary.MakeTransform` (`self.K2_GetActorLocation` (`self.K2_GetPawn`))) "Undefined" "OverrideRootScale" null null))))

(event `self.K2_OnGameClear`
  (goto _label_4))

(fn `UserConstructionScript`)